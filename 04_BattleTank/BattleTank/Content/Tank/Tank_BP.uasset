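; Player tank Blueprint that binds camera and fire input and wires its parts to the C++ Tank code.
; Aim axes orbit the camera, with yaw on an azimuth gimbal and pitch on the spring arm, both scaled by a fixed factor without delta time.
; The Fire action calls Fire, and BeginPlay passes the Barrel and Turret components to the C++ reference setters.
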(event `InputAxis|AimAzimuth`
  (params (AxisValue :type "Float (single-precision)"))
  ;[1 1 1] Input Binding Camera Rotation
  (`SceneComponent.K2_AddLocalRotation` (`self.AzimuthGimbal`) (`KismetMathLibrary.MakeRotator` 0.0 0.0 (* AxisValue 20.0)) false false))

(event `InputAction|Fire`
  (params (Key :type "Key Structure"))
  ;[1 1 1] Input Binding to Fire
  (:`Pressed`
    (`self.Fire`)))

(event `InputAxis|AimElevation`
  (params (AxisValue :type "Float (single-precision)"))
  ;[1 1 1] Input Binding Camera Rotation
  (`SceneComponent.K2_AddLocalRotation` (`self.SpringArm`) (`KismetMathLibrary.MakeRotator` 0.0 (* AxisValue 20.0)) false false))

(event `self.ReceiveBeginPlay`
  ;[1 1 1] Call 'SetBarrelReference()' in Tank.cpp and pass the Barrel in as an argument
  (`self.SetBarrelReference` (`self.Barrel`))
  (`self.SetTurretReference` (`self.Turret`)))

(fn `UserConstructionScript`)